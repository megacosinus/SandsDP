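; Inventory component that toggles the player's inventory screen with the Inventory input action.
; A FlipFlop alternates between opening and closing, setting game pause and the InventoryOpen flag each time.
; Opening creates WBP_Inventory with this component passed in and spawns BP_CharacterPreview below the world origin.
; Closing finds the top-level inventory widgets by class, removes them and destroys the preview actor.
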(event `InputAction|Inventory` :paused true
  (params (Key :type "Key Structure"))
  (:`Pressed`
    (`/Engine/EditorBlueprintResources/StandardMacros.FlipFlop`
      (:`A`
        (bind _returnvalue (`|CreateWidget` "/Game/SANDS_DP/UI/InventoryUI/WBP_Inventory.WBP_Inventory_C" (`GameplayStatics.GetPlayerController` 0) self 40.0))
        (`UserWidget.AddToViewport` _returnvalue 0)
        (`GameplayStatics.SetGamePaused` true)
        (set `self.InventoryOpen` true)
        (bind _returnvalue_2 (`|SpawnActorFromClass` "/Game/SANDS_DP/BluePrints/Inventory/BP_CharacterPreview.BP_CharacterPreview_C" (`KismetMathLibrary.MakeTransform` (0.0 0.0 -2000.0)) "Undefined" "OverrideRootScale" null null)))
      (:`B`
        (bind _foundwidgets (`WidgetBlueprintLibrary.GetAllWidgetsOfClass` "/Game/SANDS_DP/UI/InventoryUI/WBP_Inventory.WBP_Inventory_C"))
        (`Widget.RemoveFromParent` _foundwidgets)
        (`GameplayStatics.SetGamePaused` false)
        (set `self.InventoryOpen` false)
        (`Actor.K2_DestroyActor` _returnvalue_2)))))