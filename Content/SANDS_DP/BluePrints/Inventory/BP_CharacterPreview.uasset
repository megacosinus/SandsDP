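; BP_CharacterPreview is an inventory actor that renders the character for the UI preview and portrait.
; Its construction script makes the equipment meshes, from boots to helm, follow the main mesh's pose through master pose components.
; On BeginPlay, two capture components, CharacterPreviewUI and CharacterPortraitUI, are each restricted to showing only this actor's components, excluding child actors.
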(event `self.ReceiveBeginPlay`
  (`|ExecutionSequence`
    (:`then_0`
      (`SceneCaptureComponent.ShowOnlyActorComponents` (`self.CharacterPreviewUI`) self false))
    (:`then_1`
      (`SceneCaptureComponent.ShowOnlyActorComponents` (`self.CharacterPortraitUI`) self false))))

(fn `UserConstructionScript`
  (`SkinnedMeshComponent.SetLeaderPoseComponent` (`self.Boots`) (`self.MainMesh`) false)
  (`SkinnedMeshComponent.SetLeaderPoseComponent` (`self.Pants`) (`self.MainMesh`) false)
  (`SkinnedMeshComponent.SetLeaderPoseComponent` (`self.Belt`) (`self.MainMesh`) false)
  (`SkinnedMeshComponent.SetLeaderPoseComponent` (`self.Gloves`) (`self.MainMesh`) false)
  (`SkinnedMeshComponent.SetLeaderPoseComponent` (`self.Chest`) (`self.MainMesh`) false)
  (`SkinnedMeshComponent.SetLeaderPoseComponent` (`self.Armor`) (`self.MainMesh`) false)
  (`SkinnedMeshComponent.SetLeaderPoseComponent` (`self.Shoulders`) (`self.MainMesh`) false)
  (`SkinnedMeshComponent.SetLeaderPoseComponent` (`self.Helm`) (`self.MainMesh`) false))