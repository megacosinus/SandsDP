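; EQS generator that produces candidate cover points around the player for AI.
; It casts visibility traces from a ring of the given radius, spaced evenly by yaw, inward to the player's nav-projected location.
; Each blocking hit yields a point pushed out along the surface normal and raised, placing it on the obstacle's far side from the player.
; Points are gathered in a set, then added as generated vectors; the supplied context locations are unused.
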(fn `DoItemGeneration`
  (params (ContextLocations :type "Array of Vector Structure (by ref)"))
  (bind _projectedlocation (`NavigationSystemV1.K2_ProjectPointToNavigation` (`Actor.K2_GetActorLocation` (`GameplayStatics.GetPlayerCharacter` 0)) null "/Script/NavigationSystem.RecastFilter_UseDefaultArea"))
  (`KismetArrayLibrary.Array_Clear` (`self.LocationSet`))
  (for _index (range 36)
    (bind (_outhit _returnvalue) (`KismetSystemLibrary.LineTraceSingle` (+ (* (`KismetMathLibrary.GreaterGreater_VectorRotator` (1.0 0.0 0.0) (`KismetMathLibrary.MakeRotator` 0.0 0.0 (* _index 10.0))) (`self.Radius`)) _projectedlocation) _projectedlocation "TraceTypeQuery1"))
    (if _returnvalue
      (bind (_bblockinghit _binitialoverlap _time _distance _location _impactpoint _normal _impactnormal) (`GameplayStatics.BreakHitResult` _outhit))
      (`KismetArrayLibrary.Array_Add` (`self.LocationSet`) (+ _impactpoint (* _impactnormal 50.0) (0.0 0.0 100.0)))))
  (for _array_element (`self.LocationSet`)
    (`self.AddGeneratedVector` _array_element))
  (return))